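; Interactable world actor that opens the character editor when the player interacts with it.
; On interact, it casts player controller 0 to PC_CreepyToad and calls StartCharacterEditor on it.
; It reports its item type as the TryInteract state tag, while the skin and use interface functions return empty or default values.
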(event `/StateManagementSystem/Blueprints/Interface/BPI_Interact.BPI Interact`
  (bind _aspc_creepy_toad (cast `/Game/CreepyToad/Character/Blueprint/Player/PC_CreepyToad` (`GameplayStatics.GetPlayerController` 0)))
  (`/Game/CreepyToad/Character/Blueprint/Player/PC_CreepyToad.StartCharacterEditor` _aspc_creepy_toad))

(fn `BPI GetCharacterSkin`
  (returns (SkinData :type "/Game/CreepyToad/Character/Blueprint/BP_DA_CharSkin Object Reference"))
  (return null))

(fn `BPI GetCharacterSkinTag`
  (returns (Tag :type Name))
  (return "None"))

(fn `BPI GetItemType`
  (returns (Type :type "GameplayTag Structure"))
  (return (struct :`TagName` "States.Character.Interact.TryInteract")))

(fn `BPI Use`
  (returns (HungerValue :type "Float (double-precision)"))
  (return 0.0))

(fn `UserConstructionScript`)