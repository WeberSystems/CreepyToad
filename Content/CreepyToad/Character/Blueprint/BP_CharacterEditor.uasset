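; Character editor preview actor that displays a selectable character skin through a Mutable Customizable Skeletal component.
; It applies a skin on construction and BeginPlay by creating a Customizable Object instance and updating the skeletal mesh asynchronously.
; An interface event swaps skins by gender and index from the skin container's Men and Women lists.
; Another interface function returns the current skin's retarget tag.
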(event `self.ReceiveBeginPlay`
  (`self.UpdateCharacterSkin` (`self.DefaultSkin`)))

(event `/Game/CreepyToad/Character/Blueprint/BPI_Core.BPI SetNewCharacterSkinPreviewActor`
  (params (Gender :type "/Game/CreepyToad/Character/Blueprint/E_GenderTwo Enum" :default "NewEnumerator0") (Index :type Integer))
  (`self.SetNewCharacterSkin` Gender Index))

(event `/Game/CreepyToad/Character/Blueprint/BPI_Core.BPI Interact`
  (params (Actor :type "Actor Object Reference")))

(fn `BPI GetCharacterSkinTag`
  (returns (Tag :type Name))
  (bind _characterskin (`self.CharacterSkin`)
    (:`then`
      (return (`/Game/CreepyToad/Character/Blueprint/BP_DA_CharSkin.RetargetTag` _characterskin)))
    (:`else`)))

(fn `SetNewCharacterSkin`
  (params (Gender :type "/Game/CreepyToad/Character/Blueprint/E_GenderTwo Enum" :default "NewEnumerator0") (Index :type Integer))
  (bind _characterskincontainer (`self.CharacterSkinContainer`))
  (`self.UpdateCharacterSkin` (`|GetArrayItem` (select `/Game/CreepyToad/Character/Blueprint/E_GenderTwo` Gender :`NewEnumerator0` (`/Game/CreepyToad/Character/Blueprint/Data/BP_DA_SkinsContainer.Men` _characterskincontainer) :`NewEnumerator1` (`/Game/CreepyToad/Character/Blueprint/Data/BP_DA_SkinsContainer.Women` _characterskincontainer)) Index)))

(fn `UpdateCharacterSkin`
  (params (CharacterSkin :type "/Game/CreepyToad/Character/Blueprint/BP_DA_CharSkin Object Reference"))
  (bind _output_get (set `self.CharacterSkin` CharacterSkin))
  (bind _returnvalue (`CustomizableObject.CreateInstance` (`/Game/CreepyToad/Character/Blueprint/BP_DA_CharSkin.Cust` _output_get)))
  (`CustomizableSkeletalComponent.SetCustomizableObjectInstance` (`self.CustomizableSkeletal`) _returnvalue)
  (`CustomizableSkeletalComponent.UpdateSkeletalMeshAsync` (`self.CustomizableSkeletal`) true))

(fn `UserConstructionScript`
  (`self.UpdateCharacterSkin` null))