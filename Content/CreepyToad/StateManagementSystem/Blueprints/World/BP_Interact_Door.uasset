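; BP_Interact_Door is an interactable door that swings open or closed when its AC_ItemStateManager component fires OnInteracted.
; A Timeline lerps between the closed and open rotations, passing each result to OpenCloseDoor-ALL to set the Door component's relative rotation.
; DoorOpenClose picks the swing direction and matching non-spatial 2D sound, then flips when the Timeline finishes.
; Interactions are ignored while the Timeline is playing.
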(event `self.AC_ItemStateManager.OnInteracted`
  (`self.OpenCloseDoor`))

(event `OpenCloseDoor`
  (if (not (`TimelineComponent.IsPlaying` (`self.Timeline`)))
    (`|ExecutionSequence`
      (:`then_0`
        (bind (_direction _newtrack_0) (`Timeline|Timeline` :!via `PlayFromStart`)
          (:`Update`
            (`self.OpenCloseDoor - ALL` (select `bool` (`self.Door_OpenClose`) :`false` (`KismetMathLibrary.RLerp` (`self.OpenDoor_Rotation`) (`self.CloseDoor_Rotation`) _newtrack_0) :`true` (`KismetMathLibrary.RLerp` (`self.CloseDoor_Rotation`) (`self.OpenDoor_Rotation`) _newtrack_0))))
          (:`Finished`
            (if (`self.Door_OpenClose`)
              (set `self.Door_OpenClose` false)
              (else
                (set `self.Door_OpenClose` true))))))
      (:`then_1`
        (if (`self.Door_OpenClose`)
          (`GameplayStatics.PlaySound2D` "/Game/CreepyToad/StateManagementSystem/Sounds/S_Door.S_Door" 1.0 1.0 0.0 null null)
          (else
            (`GameplayStatics.PlaySound2D` "/Game/CreepyToad/StateManagementSystem/Sounds/S_DoorClose.S_DoorClose" 1.0 1.0 0.0 null null)))))))

(event `OpenCloseDoor - ALL`
  (params (NewRotation :type "Rotator Structure"))
  (`SceneComponent.K2_SetRelativeRotation` (`self.Door`) NewRotation false true))

(fn `UserConstructionScript`
  (`parent.UserConstructionScript`))