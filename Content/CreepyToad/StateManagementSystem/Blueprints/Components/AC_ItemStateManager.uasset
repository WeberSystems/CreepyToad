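; Item state manager component that responds to World.Items.States gameplay tags for destroy, interact, use and their effects.
; State activation switches on the tag to solver functions: Destroy removes the owner via a server event, Interact calls OnInteracted, and Use plays an eating sound.
; Effect solvers route through server events to multicasts, which are empty stubs.
; State cancelling has no handlers, and the additional state check defers to the parent.
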(event `self.ActivateStateSolver`
  (params (Tag :type "GameplayTag Structure"))
  (`|SwitchGameplayTag` Tag
    (:`World.Items.States.Destroy`
      (`self.DestroySolver`))
    (:`World.Items.States.DestroyEffect`
      (`self.DestroyEffectSolver`))
    (:`World.Items.States.Interact`
      (`self.InteractSolver`))
    (:`World.Items.States.InteractEffect`
      (`self.InteractEffectSolver`))
    (:`World.Items.States.Use`
      (`GameplayStatics.PlaySound2D` "/Game/CreepyToad/StateManagementSystem/Sounds/S_Eat.S_Eat" 1.0 1.0 0.0 null null))))

(event `self.CancelStateSolver`
  (params (Tag :type "GameplayTag Structure"))
  (`|SwitchGameplayTag` Tag))

(event `Server_Destroy`
  (`Actor.K2_DestroyActor` (`self.GetOwner`)))

(event `Server_DestroyEffect`
  (`self.Multicast_DestroyEffect`))

(event `Server_InteractEffect`
  (`self.Multicast_InteractEffect`))

(event `Multicast_DestroyEffect`)

(event `Multicast_InteractEffect`)

(fn `AdditionalCheckByStateType`
  (params (Tag :type "GameplayTag Structure"))
  (returns (ReturnValue :type Boolean))
  (bind _returnvalue (`parent.AdditionalCheckByStateType` Tag))
  (return _returnvalue))

(fn `DestroyEffectSolver`
  (`self.Server_DestroyEffect`))

(fn `DestroySolver`
  (`self.Server_Destroy`))

(fn `InteractEffectSolver`
  (`self.Server_InteractEffect`))

(fn `InteractSolver`
  (`self.OnInteracted`))