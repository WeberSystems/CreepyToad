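; Player state manager component that drives a Character's jump, walk speed, block, combo attack, interact, use and hunger through gameplay-tag states.
; Input functions activate or deactivate states, and solver events route each tag to its action, replicated through server and multicast events.
; Extra checks gate interact and use by line trace and item-type tag, and jump by JumpArea triggers.
; Hunger drains on a looping timer, changes on use, and prints every tick.
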(event `self.ReceiveTick`
  (params (DeltaSeconds :type "Float (single-precision)"))
  (`KismetSystemLibrary.PrintString` (`KismetStringLibrary.Conv_DoubleToString` (`self.Hunger`)) true true (struct :`R` 1.0 :`G` 0.293959 :`A` 1.0) 0.0))

(event `self.ReceiveBeginPlay`
  (bind _ascharacter (cast `Character` (`self.GetOwner`)))
  (set `self.Owner` _ascharacter)
  (for _array_element (`BlueprintGameplayTagLibrary.BreakGameplayTagContainer` (`self.StartupStates`))
    (`self.ActivateState` _array_element)))

(event `self.ActivateStateSolver`
  (params (Tag :type "GameplayTag Structure"))
  (`|SwitchGameplayTag` Tag
    (:`CharacterStates.CloseCombat.Block`
      (`self.BlockSolver` true))
    (:`CharacterStates.CloseCombat.SimpleAttack`
      (`self.AttackSolver`))
    (:`CharacterStates.Effects.HungerConsumption`
      (`self.Start Consuming Hunger Solver`))
    (:`CharacterStates.Movement.Crouch`
      (`self.WalkSolver` true))
    (:`CharacterStates.Movement.Jump`
      (`self.JumpSolver` true))
    (:`CharacterStates.UnusualSkills.Use`
      (`self.UseSolver`))
    (:`States.Character.Interact.TryInteract`
      (`self.InteractSolver`))))

(event `self.CancelStateSolver`
  (params (Tag :type "GameplayTag Structure"))
  (`|SwitchGameplayTag` Tag
    (:`CharacterStates.CloseCombat.Block`
      (`self.BlockSolver` false))
    (:`CharacterStates.Movement.Crouch`
      (`self.WalkSolver` false))
    (:`CharacterStates.Movement.Jump`
      (`self.JumpSolver` false))))

(event `Server_Jump`
  (params (Condition :type Boolean))
  ; Jumping
  (`self.Multicast_Jump` Condition))

(event `Server_Walk`
  (params (Condition :type Boolean))
  ; Walk speed
  (`self.Multicast_Walk` Condition))

(event `Multicast_Jump`
  (params (Condition :type Boolean))
  (bind _owner (`self.Owner`))
  ; Jumping
  (if Condition
    (`Character.Jump` _owner)
    (else
      (`Character.StopJumping` _owner))))

(event `Multicast_Walk`
  (params (Condition :type Boolean))
  ; Walk speed
  (set `CharacterMovementComponent.MaxWalkSpeed` (select `bool` Condition :`false` 500.0 :`true` 100.0 :!type "Float (single-precision)") (`Character.CharacterMovement` (`self.Owner`))))

(event `Server_Attack`
  ; Attack
  (`self.Multicast_Attack`))

(event `Server_Block`
  (params (Condition :type Boolean))
  ; Block
  (`self.Multicast_Block` Condition))

(event `Multicast_Attack`
  ; Attack
  (`|PlayMontage` (`Character.Mesh` (`self.Owner`)) "/Game/CreepyToad/StateManagementSystem/Meshes/Mannequins/Animations/AM_Combo.AM_Combo"
    (:`OnCompleted`
      (`self.DeactivateState` (struct :`TagName` "CharacterStates.CloseCombat.SimpleAttack")))))

(event `Multicast_Block`
  (params (Condition :type Boolean))
  ; Block
  (bind _asabp_manny_plugin (cast `/Game/CreepyToad/StateManagementSystem/Meshes/Mannequins/Animations/ABP_MannyPlugin` (`SkeletalMeshComponent.GetAnimInstance` (`Character.Mesh` (`self.Owner`)))))
  (`/Game/CreepyToad/StateManagementSystem/Meshes/Mannequins/Animations/ABP_MannyPlugin.SetBlockState` _asabp_manny_plugin Condition))

(event `Server_Interact`
  (params (InteractActor :type "Actor Object Reference"))
  (bind _output_get (set `self.LastInteractActor` InteractActor))
  (message `/Game/CreepyToad/StateManagementSystem/Blueprints/Interface/BPI_Interact.BPI Interact` _output_get (`self.GetOwner`)))

(event `Server_Use`
  (params (LastInteractActor :type "Actor Object Reference"))
  (bind _output_get (set `self.LastInteractActor` LastInteractActor))
  (bind _hungervalue (message `/Game/CreepyToad/StateManagementSystem/Blueprints/Interface/BPI_Interact.BPI Use` _output_get))
  (`self.HungerChanged - OC` (`KismetMathLibrary.FClamp` (+ _hungervalue (`self.Hunger`)) 0.0 100.0)))

(event `Start Consuming Hunger - OC`
  (`self.Start Consuming Hunger`))

(event `HungerChanged - OC`
  (params (Value :type "Float (double-precision)"))
  (set `self.Hunger` Value))

(fn `AC Interact`
  (returns (ReturnValue :type Boolean))
  (bind _returnvalue (`GameplayStatics.GetPlayerController` 0))
  (bind _returnvalue_2 (`Actor.K2_GetActorLocation` (`PlayerController.PlayerCameraManager` _returnvalue)))
  (bind (_outhit _returnvalue_3) (`KismetSystemLibrary.LineTraceSingle` _returnvalue_2 (+ _returnvalue_2 (* (`Actor.GetActorForwardVector` _returnvalue) 500)) "TraceTypeQuery3"))
  (if _returnvalue_3
    (bind (_bblockinghit _binitialoverlap _time _distance _location _impactpoint _normal _impactnormal _physmat _hitactor) (`GameplayStatics.BreakHitResult` _outhit))
    (`/Engine/EditorBlueprintResources/StandardMacros.IsValid` _hitactor
      (:`Is Valid`
        (bind _output_get (set `self.LastInteractActor` _hitactor))
        (bind _type (message `/Game/CreepyToad/StateManagementSystem/Blueprints/Interface/BPI_Interact.BPI GetItemType` _output_get))
        (return (`BlueprintGameplayTagLibrary.HasTag` (`self.InteractTypes`) _type))))))

(fn `AC Jump`
  (returns (ReturnValue :type Boolean))
  (bind _ascharacter (cast `Character` (`self.GetOwner`)))
  (for _array_element (`PrimitiveComponent.GetOverlappingActors` (`Character.CapsuleComponent` _ascharacter) "/Script/Engine.TriggerBox")
    (if (`KismetArrayLibrary.Array_Contains` (`Actor.Tags` _array_element) "JumpArea")
      (return true)))
  (return false))

(fn `AC Use`
  (returns (ReturnValue :type Boolean))
  (bind _returnvalue (`GameplayStatics.GetPlayerController` 0))
  (bind _returnvalue_2 (`Actor.K2_GetActorLocation` (`PlayerController.PlayerCameraManager` _returnvalue)))
  (bind (_outhit _returnvalue_3) (`KismetSystemLibrary.LineTraceSingle` _returnvalue_2 (+ _returnvalue_2 (* (`Actor.GetActorForwardVector` _returnvalue) 500)) "TraceTypeQuery1"))
  (if _returnvalue_3
    (bind (_bblockinghit _binitialoverlap _time _distance _location _impactpoint _normal _impactnormal _physmat _hitactor) (`GameplayStatics.BreakHitResult` _outhit))
    (`/Engine/EditorBlueprintResources/StandardMacros.IsValid` _hitactor
      (:`Is Valid`
        (bind _output_get (set `self.LastInteractActor` _hitactor))
        (bind _type (message `/Game/CreepyToad/StateManagementSystem/Blueprints/Interface/BPI_Interact.BPI GetItemType` _output_get))
        (return (`BlueprintGameplayTagLibrary.HasTag` (`self.UseTypes`) _type))))))

(fn `AdditionalCheckByStateType`
  (params (Tag :type "GameplayTag Structure"))
  (returns (ReturnValue :type Boolean))
  (`|SwitchGameplayTag` Tag
    (:`States.Character.Interact.TryInteract`
      (return (`self.AC Interact`)))
    (:`CharacterStates.UnusualSkills.Use`
      (return (`self.AC Use`)))
    (:`CharacterStates.Movement.Jump`
      (return (`self.AC Jump`)))))

(fn `AttackSolver`
  (`/Engine/EditorBlueprintResources/ActorComponentMacros.Switch Has Authority`
    (:`Authority`
      (`self.Multicast_Attack`))
    (:`Remote`
      (`self.Server_Attack`))))

(fn `BlockSolver`
  (params (Condition :type Boolean))
  (`/Engine/EditorBlueprintResources/ActorComponentMacros.Switch Has Authority`
    (:`Authority`
      (`self.Multicast_Block` Condition))
    (:`Remote`
      (`self.Server_Block` Condition))))

(fn `BPI GetItemType`
  (returns (Type :type "GameplayTag Structure"))
  (return))

(fn `BPI Use`
  (returns (HungerValue :type "Float (double-precision)"))
  (return 0.0))

(fn `End Hunger Consumption Process`
  (`KismetSystemLibrary.K2_ClearAndInvalidateTimerHandle` (`self.HungerConsumptionTimer`)))

(fn `Hunger Changed`
  (params (Hunger :type "Float (double-precision)"))
  (bind _output_get (set `self.Hunger` Hunger))
  (`self.HungerChanged - OC` _output_get))

(fn `Hunger Consumption Process`
  (`self.Hunger Changed` (`KismetMathLibrary.FClamp` (- (`self.Hunger`) 0.1) 0.0 100.0)))

(fn `IA_Attack`
  (`self.ActivateState` (struct :`TagName` "CharacterStates.CloseCombat.SimpleAttack")))

(fn `IA_BlockState`
  (params (Condition :type Boolean))
  (if Condition
    (`self.ActivateState` (struct :`TagName` "CharacterStates.CloseCombat.Block"))
    (else
      (`self.DeactivateState` (struct :`TagName` "CharacterStates.CloseCombat.Block")))))

(fn `IA_Interact`
  (`self.ActivateState` (struct :`TagName` "States.Character.Interact.TryInteract")))

(fn `IA_JumpState`
  (params (Condition :type Boolean))
  (if Condition
    (`self.ActivateState` (struct :`TagName` "CharacterStates.Movement.Jump"))
    (else
      (`self.DeactivateState` (struct :`TagName` "CharacterStates.Movement.Jump")))))

(fn `IA_Use`
  (`self.ActivateState` (struct :`TagName` "CharacterStates.UnusualSkills.Use")))

(fn `IA_WalkState`
  (if (`self.DoesStateExists` (struct :`TagName` "CharacterStates.Movement.Walk"))
    (`self.DeactivateState` (struct :`TagName` "CharacterStates.Movement.Walk"))
    (else
      (`self.ActivateState` (struct :`TagName` "CharacterStates.Movement.Walk")))))

(fn `InteractSolver`
  (bind _lastinteractactor (`self.LastInteractActor`)
    (:`then`
      (`self.Server_Interact` _lastinteractactor))
    (:`else`)))

(fn `JumpSolver`
  (params (Condition :type Boolean))
  (`/Engine/EditorBlueprintResources/ActorComponentMacros.Switch Has Authority`
    (:`Authority`
      (`self.Multicast_Jump` Condition))
    (:`Remote`
      (`self.Server_Jump` Condition))))

(fn `Start Consuming Hunger`
  (`self.End Hunger Consumption Process`)
  (bind _returnvalue (`KismetSystemLibrary.K2_SetTimerDelegate` (`|CreateDelegate` :!event `Hunger Consumption Process`) 1.0 true))
  (set `self.HungerConsumptionTimer` _returnvalue))

(fn `Start Consuming Hunger Solver`
  (if (`Pawn.IsLocallyControlled` (`self.Owner`))
    (`self.Start Consuming Hunger - OC`)))

(fn `UseSolver`
  (bind _lastinteractactor (`self.LastInteractActor`)
    (:`then`
      (`self.Server_Use` _lastinteractactor))
    (:`else`)))

(fn `WalkSolver`
  (params (Condition :type Boolean))
  (`/Engine/EditorBlueprintResources/ActorComponentMacros.Switch Has Authority`
    (:`Authority`
      (`self.Multicast_Walk` Condition))
    (:`Remote`
      (`self.Server_Walk` Condition))))