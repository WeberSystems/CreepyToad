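; BP_CharacterEditorInteract is a world interactable that opens the character editor for the player who uses it.
; The interact interface event passes the instigator to a multicast, which calls StartCharacterEditor on that character's PC_BaseController only where it is the local player controller.
; It reports its item type as the TryInteract state tag; the other interface functions return empty defaults.
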(event `/Game/Characters/Blueprint/Interface/BPI_Interact.BPI Interact`
  (params (Insigator :type "Actor Object Reference"))
  (`self.Multicast_Interact` Insigator))

(event `Multicast_Interact`
  (params (Object :type "Object Object Reference"))
  (bind _ascharacter (cast `Character` Object))
  (bind _aspc_base_controller (cast `/Game/Characters/Blueprint/Player/PC_BaseController` (`Pawn.GetController` _ascharacter)))
  (if (`Controller.IsLocalPlayerController` _aspc_base_controller)
    (`/Game/Characters/Blueprint/Player/PC_BaseController.StartCharacterEditor` _aspc_base_controller)))

(fn `BPI GetCharacterSkin`
  (returns (SkinData :type "/Game/Characters/Blueprint/BP_DA_CharSkin Object Reference"))
  (return null))

(fn `BPI GetCharacterSkinTag`
  (returns (Tag :type Name))
  (return "None"))

(fn `BPI GetItemType`
  (returns (Type :type "GameplayTag Structure"))
  (return (struct :`TagName` "States.Character.Interact.TryInteract")))

(fn `BPI Use`
  (returns (HungerValue :type "Float (double-precision)"))
  (return 0.0))

(fn `UserConstructionScript`)