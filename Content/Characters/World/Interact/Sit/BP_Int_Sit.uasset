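; BP_Int_Sit is a sittable chair actor that characters query through a Blueprint interface.
; The interface returns the chair mesh, the SitPlace reference and the world transform of StandPlace.
; An occupancy flag, SomeoneSitOnChair, is set through an interface event and inverted to report whether the chair can be sat on.
; The actor only holds this data and state, with no sitting logic or active Tick of its own.
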(event `/Game/Characters/Blueprint/Interface/BPI_Interact.BPI SetSomeoneSitOnChair`
  (params (State :type Boolean))
  (set `self.SomeoneSitOnChair` State))

(fn `BPI CanSitOnChair`
  (returns (ReturnValue :type Boolean))
  (return (not (`self.SomeoneSitOnChair`))))

(fn `BPI GetChairMesh`
  (returns (MeshComponent :type "StaticMeshComponent Object Reference"))
  (return (`self.StaticMesh`)))

(fn `BPI GetSitPlace`
  (returns (Place :type "PrimitiveComponent Object Reference"))
  (return (`self.SitPlace`)))

(fn `BPI GetStandChairPlace`
  (returns (Position :type "Transform Structure"))
  (return (`SceneComponent.K2_GetComponentToWorld` (`self.StandPlace`))))

(fn `UserConstructionScript`
  (`parent.UserConstructionScript`))