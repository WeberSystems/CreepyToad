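; BP_InteractPhysic is an interactable physics object that tracks which player is holding it.
; Its only active logic, the Multicast_ControlHeldByRef event, stores the HeldByPlayer reference and applies a caller-supplied collision response to the static mesh's Pawn channel.
; The caller therefore decides how the object collides with pawns as its holder changes.
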(event `Multicast_ControlHeldByRef`
  (params (HeldByPlayer :type "Character Object Reference") (NewResponse :type "ECollisionResponse Enum" :default "ECR_Ignore"))
  (set `self.HeldByPlayer` HeldByPlayer)
  (`PrimitiveComponent.SetCollisionResponseToChannel` (`self.StaticMesh`) "ECC_Pawn" NewResponse))

(fn `UserConstructionScript`
  (`parent.UserConstructionScript`))