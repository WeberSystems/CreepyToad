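; Interactable actor that a player swings around its yaw axis by moving the mouse, within angle limits.
; The interact interface call toggles Tick on the controlling client, capturing the starting mouse direction and, on release, the pivot's yaw.
; Each tick measures the signed horizontal angle between deprojected mouse directions, adjusted for player side and sensitivity.
; The clamped angle goes to the server, and CurrentAngle's OnRep rotates the Pivot.
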(event `self.ReceiveTick`
  (params (DeltaSeconds :type "Float (single-precision)"))
  (`parent.ReceiveTick` DeltaSeconds)
  (if (`Pawn.IsLocallyControlled` (`self.PlayerInteract`))
    (`self.Client_UpdatePivot`)))

(event `Client_Control Interact State`
  (params (InputPin :type "Character Object Reference") (Condition :type Boolean))
  (bind (_relativerotation_roll _relativerotation_pitch _relativerotation_yaw) (`KismetMathLibrary.BreakRotator` (`SceneComponent.RelativeRotation` (`self.Pivot`))))
  (if Condition
    (bind _asbp_base_character (cast `/Game/Characters/Blueprint/Player/BP_BaseCharacter` InputPin))
    (bind _output_get (set `self.PlayerInteract` _asbp_base_character))
    (set `self.CameraReference` (`/Game/Characters/Blueprint/Player/BP_BaseCharacter.FirstPersonCamera` _output_get))
    (set `self.StartDirection` (`KismetMathLibrary.Normal` (`.WorldDirection` (`GameplayStatics.DeprojectScreenToWorld` (`GameplayStatics.GetPlayerController` 0) (`/Game/Characters/Blueprint/Player/BP_BaseCharacter.MouseAxis` (`self.PlayerInteract`))))))
    (set `self.SideSign` (`KismetMathLibrary.SignOfFloat` (`KismetMathLibrary.Dot_VectorVector` (- (`self.K2_GetActorLocation` (`self.PlayerInteract`)) (`self.K2_GetActorLocation`)) (`self.GetActorRightVector`))))
    (`self.SetActorTickEnabled` true)
    (else
      (`self.SetActorTickEnabled` false)
      (set `self.PlayerInteract` null)
      (set `self.CameraReference` null)
      (set `self.StartAngleYaw` _relativerotation_yaw)
      (set `self.StartDirection` (0.0 0.0 0.0)))))

(event `/Game/Characters/Blueprint/Interface/BPI_Interact.BPI ControlInteractState`
  (params (CharacterRef :type "Character Object Reference") (State :type Boolean))
  (`self.Client_Control Interact State ` CharacterRef State))

(event `Client_UpdatePivot`
  (`self.UpdatePivot`))

(event `Server_UpdatePivot`
  (params (CurrentAngle :type "Float (double-precision)"))
  (set `self.CurrentAngle` CurrentAngle))

(fn `OnRep_CurrentAngle`
  (`SceneComponent.K2_SetRelativeRotation` (`self.Pivot`) (`KismetMathLibrary.MakeRotator` 0.0 0.0 (`self.CurrentAngle`)) false false))

(fn `UpdatePivot`
  (locals (CamRight :type "Vector Structure") (CamUp :type "Vector Structure") (Axis :type "Vector Structure" :default (0.0 0.0 0.0)) (DotRight :type "Float (double-precision)") (DotUp :type "Float (double-precision)") (Delta :type "Float (double-precision)") (CurrentDirection :type "Vector Structure" :default (0.0 0.0 0.0)) (ProjectedStart :type "Vector Structure") (ProjectedCurrent :type "Vector Structure") (Dot :type "Float (double-precision)" :default 0.0) (Cross :type "Vector Structure" :default (0.0 0.0 0.0)) (MouseWorldDir :type "Vector Structure" :default (0.0 0.0 0.0)) (A :type "Vector Structure" :default (0.0 0.0 0.0)) (B :type "Vector Structure" :default (0.0 0.0 0.0)))
  (bind (_cross_x _cross_y _cross_z) (`KismetMathLibrary.BreakVector` (`local.Cross`)))
  (set `local.MouseWorldDir` (`.WorldDirection` (`GameplayStatics.DeprojectScreenToWorld` (`GameplayStatics.GetPlayerController` 0) (`/Game/Characters/Blueprint/Player/BP_BaseCharacter.MouseAxis` (`self.PlayerInteract`)))))
  (set `local.A` (`KismetMathLibrary.ProjectVectorOnToPlane` (`self.StartDirection`) (0.0 0.0 1.0)))
  (set `local.B` (`KismetMathLibrary.ProjectVectorOnToPlane` (`local.MouseWorldDir`) (0.0 0.0 1.0)))
  (set `local.Cross` (`KismetMathLibrary.Cross_VectorVector` (`local.A`) (`local.B`)))
  (set `local.Dot` (`KismetMathLibrary.Dot_VectorVector` (`local.A`) (`local.B`)))
  (set `local.Delta` (`KismetMathLibrary.DegAtan2` _cross_z (`local.Dot`)))
  (`self.Server_UpdatePivot` (`KismetMathLibrary.FClamp` (+ (`self.StartAngleYaw`) (* (`local.Delta`) (`self.Direction`) (`self.Sensitivity`) (`KismetMathLibrary.SignOfFloat` (`KismetMathLibrary.Dot_VectorVector` (- (`self.K2_GetActorLocation` (`self.PlayerInteract`)) (`self.K2_GetActorLocation`)) (`self.GetActorRightVector`))))) (`self.MinAngle`) (`self.MaxAngle`))))

(fn `UserConstructionScript`
  (`parent.UserConstructionScript`))