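; BP_InteractMaster is a master Blueprint for interactable world items, backed by data table entries.
; On BeginPlay it looks up its ItemRow handle and caches the found row as ItemData.
; Interface functions expose that data and a fixed interact type.
; GetItemType and Use are placeholders returning empty or zero values, and the construction script, overlap and tick events do nothing.
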(event `self.ReceiveBeginPlay`
  (bind (_datatable _rowname) (break `DataTableRowHandle` (`self.ItemRow`)))
  (bind _returnvalue (`|GetDataTableRow` _datatable _rowname)
    (:`then`
      (set `self.ItemData` _returnvalue))))

(fn `BPI GetInteractType`
  (returns (EInteractType :type "/Game/Characters/Blueprint/Interface/EInteractType Enum"))
  (return "NewEnumerator0"))

(fn `BPI GetItemData`
  (returns (ItemData :type "/Game/Blueprints/Data/FItemData Structure"))
  (return (`self.ItemData`)))

(fn `BPI GetItemType`
  (returns (Type :type "GameplayTag Structure"))
  (return))

(fn `BPI Use`
  (returns (HungerValue :type "Float (double-precision)"))
  (return 0.0))

(fn `UserConstructionScript`)