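; BP_Int_Openable is an interactable world object that toggles between open and closed, prompting "Open" or "Close" accordingly.
; Interaction flips Open, whose OnRep sets the Openable component's rotation and plays a sound parameterized by that state.
; With SmoothOpen, a timeline interpolates the rotation at SmoothOpenRate; an interrupted swing restarts from the mirrored playback position to reverse mid-motion.
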(event `self.ReceiveBeginPlay`
  (`parent.ReceiveBeginPlay`)
  (`TimelineComponent.SetPlayRate` (`self.OpenClose`) (`self.SmoothOpenRate`)))

(event `/Game/Characters/Blueprint/Interface/BPI_Interact.BPI Interact`
  (params (Insigator :type "Actor Object Reference"))
  (`parent.BPI Interact` Insigator)
  (set `self.Open` (not (`self.Open`))))

(event `Multicast_UpdateState`
  (params (State :type Boolean))
  (set `self.Open` State))

(event `OpenCapSmooth`
  (if (`TimelineComponent.IsPlaying` (`self.OpenClose`))
    (`TimelineComponent.Stop` (`self.OpenClose`))
    (set `self.StartTime` (- 1.0 (`TimelineComponent.GetPlaybackPosition` (`self.OpenClose`))))
    (else
      (set `self.StartTime` 0.0)))
  (`|ExecutionSequence`
    (:`then_0`
      (bind (_direction _newtrack_0) (`Timeline|OpenClose` :`NewTime` (`self.StartTime`) :!via `SetNewTime` :!label _label)
        (:`Update`
          (`SceneComponent.K2_SetRelativeRotation` (`self.Openable`) (`KismetMathLibrary.RLerp` (select `bool` (`self.Open`) :`false` (`self.OpenAngle`) :`true` (`self.CloseAngle`)) (select `bool` (`self.Open`) :`false` (`self.CloseAngle`) :`true` (`self.OpenAngle`)) _newtrack_0) false true))))
    (:`then_1`
      (goto _label))))

(fn `BPI CanSitOnChair`
  (returns (ReturnValue :type Boolean))
  (return false))

(fn `BPI GetAdvancedInteractText`
  (returns (Text :type Text))
  (return (select `bool` (`self.Open`) :`false` "Open" :`true` "Close" :!type "Text")))

(fn `BPI GetChairMesh`
  (returns (MeshComponent :type "StaticMeshComponent Object Reference"))
  (return (`self.StaticMesh`)))

(fn `BPI GetSitPlace`
  (returns (Place :type "PrimitiveComponent Object Reference"))
  (return null))

(fn `BPI GetStandChairPlace`
  (returns (Position :type "Transform Structure"))
  (return))

(fn `OnRep_Open`
  (if (`self.SmoothOpen`)
    (`self.OpenCapSmooth`)
    (else
      (`SceneComponent.K2_SetRelativeRotation` (`self.Openable`) (select `bool` (`self.Open`) :`false` (`self.CloseAngle`) :`true` (`self.OpenAngle`)) false false)))
  (`AudioComponent.SetBoolParameter` (`self.InteractSound`) "Open" (`self.Open`))
  (`AudioComponent.Play` (`self.InteractSound`) 0.0))

(fn `UserConstructionScript`
  (`parent.UserConstructionScript`))