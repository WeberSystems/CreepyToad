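; Player character component that runs a gameplay-tag state machine for movement, interaction and physics object grabbing.
; DT_CharacterStates rows define each state's required, forbidden and chained tags, checked before activation.
; Solvers dispatch state changes to server and multicast events, and the active tag container is replicated by RPC.
; A looping camera trace updates interaction UI and target; grabbed items follow a PhysicsHandle on Tick and can be rotated, moved or thrown.
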(event `self.ReceiveTick`
  (params (DeltaSeconds :type "Float (single-precision)"))
  (`|ExecutionSequence`
    (:`then_0`
      (for _array_element (`BlueprintGameplayTagLibrary.BreakGameplayTagContainer` (`self.GameplayTagsContainer`))
        (`KismetSystemLibrary.PrintString` (`KismetStringLibrary.Conv_NameToString` (`BlueprintGameplayTagLibrary.GetTagName` _array_element)) true true (struct :`R` 1.0 :`G` 0.168575 :`A` 1.0) 0.0)))
    (:`then_1`
      (`self.ControlGrabbedComponentPosition`))))

(event `self.ReceiveBeginPlay`
  (`KismetSystemLibrary.Delay` 0.2)
  (bind _asbp_base_character (cast `/Game/Characters/Blueprint/Player/BP_BaseCharacter` (`self.GetOwner`)))
  (bind _output_get (set `self.Owner` _asbp_base_character))
  (bind _aspc_base_controller (cast `/Game/Characters/Blueprint/Player/PC_BaseController` (`Pawn.GetController` _output_get)))
  (set `self.PC Base Controller` _aspc_base_controller)
  (set `self.Physics Handle` (`/Game/Characters/Blueprint/Player/BP_BaseCharacter.PhysicsHandle` (`self.Owner`)))
  (set `self.Attach Grab Item Place` (`/Game/Characters/Blueprint/Player/BP_BaseCharacter.AttachGrabItemPlace` (`self.Owner`)))
  (`self.ActivateStates` (`BlueprintGameplayTagLibrary.BreakGameplayTagContainer` (`self.StartupStates`))))

(event `Server_Jump`
  (params (Condition :type Boolean))
  ; Jumping
  (`self.Multicast_Jump` Condition))

(event `Multicast_Jump`
  (params (Condition :type Boolean))
  (bind _owner (`self.Owner`))
  ; Jumping
  (if Condition
    (`Character.Jump` _owner)
    (else
      (`Character.StopJumping` _owner))))

(event `Server_Crouch`
  (params (Condition :type Boolean))
  ; Crouch
  (`self.Multicast_Crouch` Condition))

(event `Server_RunState`
  (params (Condition :type Boolean))
  (`self.Multicast_RunState` Condition))

(event `Multicast_Crouch`
  (params (Condition :type Boolean))
  ; Crouch
  (if Condition
    (`Character.Crouch` (`self.Owner`))
    (else
      (`Character.UnCrouch` (`self.Owner`)))))

(event `Multicast_RunState`
  (params (Condition :type Boolean))
  (bind _character_movement (`self.GetCharacterMovement`))
  (if Condition
    (set `CharacterMovementComponent.MaxWalkSpeed` 380.0 _character_movement)
    (else
      (set `CharacterMovementComponent.MaxWalkSpeed` 160.0 _character_movement))))

(event `Server_Interact`
  (params (InteractActor :type "Actor Object Reference") (InteractKey :type "/Game/Characters/World/Interact/EInteractActionKey Enum" :default "NewEnumerator3"))
  (bind _output_get (set `self.LastInteractActor` InteractActor))
  (bind _einteractdata (message `/Game/Characters/Blueprint/Interface/BPI_Interact.BPI GetInteractType` _output_get InteractKey))
  (bind (_action _customstate) (break `/Game/Characters/World/Interact/FInteractActionByInput` _einteractdata))
  (switch `/Game/Characters/World/Interact/EInteractAction` _action
    (:`NewEnumerator1`
      (message `/Game/Characters/Blueprint/Interface/BPI_Interact.BPI Interact` (`self.LastInteractActor`) (`self.GetOwner`))
      (`self.Deactivate State` (struct :`TagName` "States.Character.Interact.TryInteract")))
    (:`NewEnumerator2`
      (`self.Activate State` _customstate)
      (`KismetSystemLibrary.PrintString` (`BlueprintGameplayTagLibrary.GetDebugStringFromGameplayTag` _customstate)))
    (:`NewEnumerator3`
      (`self.Deactivate State` _customstate))
    (:`NewEnumerator4`
      (`self.Activate State` (struct :`TagName` "States.Character.Interact.GrabObject"))
      (`self.Deactivate State` (struct :`TagName` "States.Character.Interact.TryInteract")))))

(event `Server_LeftMouseButton`
  (if (`self.Does State Exist` (struct :`TagName` "States.Character.Interact.GrabObject"))
    (set `self.DropGrabbedObjectNeedImpulse` false)
    (`self.Deactivate State` (struct :`TagName` "States.Character.Interact.GrabObject"))
    (else
      (`self.Activate State` (struct :`TagName` "States.Character.Interact.LMBInteract")))))

(event `Server_RightMouseButton`
  (if (`self.Does State Exist` (struct :`TagName` "States.Character.Interact.GrabObject"))
    (set `self.DropGrabbedObjectNeedImpulse` true)
    (`self.Deactivate State` (struct :`TagName` "States.Character.Interact.GrabObject"))
    (else
      (`self.Activate State` (struct :`TagName` "States.Character.Interact.RMBInteract")))))

(event `Client_SetGrabObjectRef`
  (params (HeldItem :type "/Game/Characters/World/Interact/BP_InteractPhysic Object Reference"))
  (set `self.HeldItem` HeldItem))

(event `Server_SetHoldDistanceGrabbedObject`
  (params (Alpha :type "Float (double-precision)"))
  (bind (_holddistancegrabbedobjectclamp_x _holddistancegrabbedobjectclamp_y) (`KismetMathLibrary.BreakVector2D` (`self.HoldDistanceGrabbedObjectClamp`)))
  (set `self.GrabbedComponentHoldDistance` (`KismetMathLibrary.FClamp` (+ (* Alpha (`self.SetHoldDistanceGrabbedObjectAlpha`)) (`self.GrabbedComponentHoldDistance`)) _holddistancegrabbedobjectclamp_x _holddistancegrabbedobjectclamp_y)))

(event `Server_SetGrabbedObjectRotation`
  (params (HeldActorRotation :type "Rotator Structure"))
  (set `self.HeldActorRotation` HeldActorRotation))

(event `Replicate_RealTime Character State - Server`
  (params (GameplayTagsContainer :type "GameplayTagContainer Structure"))
  (`self.Replicate_RealTime Character State - ALL` GameplayTagsContainer))

(event `Replicate_RealTime Character State - ALL`
  (params (GameplayTagsContainer :type "GameplayTagContainer Structure"))
  (set `self.GameplayTagsContainer` GameplayTagsContainer))

(fn `AC GrabObject`
  (returns (ReturnValue :type Boolean))
  (bind _lastinteractactor (`self.LastInteractActor`)
    (:`then`
      (bind _asbp_interact_physic (cast `/Game/Characters/World/Interact/BP_InteractPhysic` _lastinteractactor))
      (return (not (`KismetSystemLibrary.IsValid` (`/Game/Characters/World/Interact/BP_InteractPhysic.HeldByPlayer` _asbp_interact_physic)))))
    (:`else`)))

(fn `AC Interact`
  (returns (ReturnValue :type Boolean))
  (bind _returnvalue (`GameplayStatics.GetPlayerController` 0))
  (bind _returnvalue_2 (`Actor.K2_GetActorLocation` (`PlayerController.PlayerCameraManager` _returnvalue)))
  (bind (_outhit _returnvalue_3) (`KismetSystemLibrary.LineTraceSingle` :`Start` _returnvalue_2 :`End` (+ _returnvalue_2 (* (`Actor.GetActorForwardVector` _returnvalue) 500)) :`TraceChannel` (`self.Trace Channel Interact`) :`DrawDebugType` "ForDuration"))
  (if _returnvalue_3
    (bind (_bblockinghit _binitialoverlap _time _distance _location _impactpoint _normal _impactnormal _physmat _hitactor) (`GameplayStatics.BreakHitResult` _outhit))
    (`/Engine/EditorBlueprintResources/StandardMacros.IsValid` _hitactor
      (:`Is Valid`
        (bind _output_get (set `self.LastInteractActor` _hitactor))
        (return true)))))

(fn `Activate State`
  (params (Tag :type "GameplayTag Structure"))
  (returns (`Return Value` :type Boolean))
  (locals (`ActivateStates After Activating` :type "GameplayTagContainer Structure") (`CancelStates After Activating` :type "GameplayTagContainer Structure") (CurrentState :type "GameplayTag Structure") (`Activate States Before Activating` :type "GameplayTagContainer Structure" :default (struct)) (`Cancel States Before Activating` :type "GameplayTagContainer Structure") (Result :type "/Game/Characters/Blueprint/Data/Tables/S_AC_StateContainer Structure"))
  (bind _output_get (set `local.CurrentState` Tag))
  (bind _output_get_2 (set `local.Result` (`self.State Machine Solver` _output_get)))
  (bind (_result _activatestatesafteractivating _activatestatesbeforeactivating _cancelstatesbeforeactivating _cancelstatesafteractivating) (break `/Game/Characters/Blueprint/Data/Tables/S_AC_StateContainer` _output_get_2))
  (if _result
    (set `local.ActivateStates After Activating` _activatestatesafteractivating)
    (set `local.Activate States Before Activating` _activatestatesbeforeactivating)
    (set `local.Cancel States Before Activating` _cancelstatesbeforeactivating)
    (set `local.CancelStates After Activating` _cancelstatesafteractivating)
    (`|ExecutionSequence`
      (:`then_0`
        (for _array_element (`BlueprintGameplayTagLibrary.BreakGameplayTagContainer` (`local.Activate States Before Activating`))
          (`self.Activate State` _array_element))
        (`self.Deactivate States` (`BlueprintGameplayTagLibrary.BreakGameplayTagContainer` (`local.Cancel States Before Activating`)))
        (`self.Control Real Time Character State` "NewEnumerator0" (`local.CurrentState`))
        (`self.Replicate Real Time Character State - Solver` (`self.GameplayTagsContainer`))
        (`self.Activate State Solver` (`local.CurrentState`))
        (`self.Deactivate States` (`BlueprintGameplayTagLibrary.BreakGameplayTagContainer` (`local.CancelStates After Activating`)))
        (for _array_element_2 (`BlueprintGameplayTagLibrary.BreakGameplayTagContainer` (`local.ActivateStates After Activating`))
          (`self.Activate State` _array_element_2)))
      (:`then_1`
        (if (`.RemoveAfterActivation_19_ABD9140F495077E46B049FA00F448BCD` (break `/Game/Characters/Blueprint/Data/Tables/S_AC_StateContainer` (`local.Result`)))
          (`self.Deactivate State` (`local.CurrentState`))))
      (:`then_2`
        (return true)))
    (else
      (return false))))

(fn `Activate State Solver`
  (params (Tag :type "GameplayTag Structure"))
  (`|SwitchGameplayTag` Tag
    (:`States.Character.Movement.Crouch`
      (`self.CrouchSolver` true))
    (:`States.Character.Movement.Jump`
      (`self.JumpSolver` true))
    (:`States.Character.Interact.TryInteract`
      (`self.InteractSolver` "NewEnumerator0"))
    (:`States.Character.Movement.Run`
      (`self.RunSolver` true))
    (:`States.Character.Interact.CheckInteractActorsTrace`
      (`self.CheckInteractActorsTraceSolver` true))
    (:`States.Character.Interact.GrabObject`
      (`self.GrabObjectSolver` true))
    (:`States.Character.Interact.LMBInteract`
      (`self.InteractSolver` "NewEnumerator1"))
    (:`States.Character.Interact.RMBInteract`
      (`self.InteractSolver` "NewEnumerator2"))))

(fn `ActivateStates`
  (params (Tags :type "Array of GameplayTag Structure"))
  (if (`KismetArrayLibrary.Array_IsNotEmpty` Tags)
    (for _array_element Tags
      (`self.Activate State` _array_element)))
  (return))

(fn `Additional Check By State Type`
  (params (NewTag :type "GameplayTag Structure"))
  (returns (Result :type Boolean))
  (`|SwitchGameplayTag` NewTag
    (:`States.Character.Interact.TryInteract`
      (return (`self.AC Interact`)))
    (:`States.Character.Interact.GrabObject`
      (return (`self.AC GrabObject`)))))

(fn `BPI GetInteractType`
  (params (InteractKey :type "/Game/Characters/World/Interact/EInteractActionKey Enum" :default "NewEnumerator3"))
  (returns (EInteractData :type "/Game/Characters/World/Interact/FInteractActionByInput Structure"))
  (return))

(fn `BPI GetItemData`
  (returns (ItemData :type "/Game/Blueprints/Data/FItemData Structure"))
  (return))

(fn `BPI GetItemType`
  (returns (Type :type "GameplayTag Structure"))
  (return))

(fn `BPI Use`
  (returns (HungerValue :type "Float (double-precision)"))
  (return 0.0))

(fn `Cancel State Solver`
  (params (Tag :type "GameplayTag Structure"))
  (`|SwitchGameplayTag` Tag
    (:`States.Character.Movement.Crouch`
      (`self.CrouchSolver` false))
    (:`States.Character.Movement.Jump`
      (`self.JumpSolver` false))
    (:`States.Character.Movement.Run`
      (`self.RunSolver` false))
    (:`States.Character.Interact.CheckInteractActorsTrace`
      (`self.CheckInteractActorsTraceSolver` false))
    (:`States.Character.Interact.GrabObject`
      (`self.GrabObjectSolver` false))))

(fn `CheckInteractActorsTrace`
  (locals (HitActorTemp :type "Actor Object Reference"))
  (bind (_hitactor _returnvalue) (`self.InteractTrace`))
  (set `local.HitActorTemp` _hitactor)
  (if _returnvalue
    (`local.HitActorTemp`
      (:`then`
        (`self.LastCheckInteractActor`
          (:`then`
            (if (!= (`self.LastCheckInteractActor`) (`local.HitActorTemp`))
              (if (`KismetSystemLibrary.DoesImplementInterface` (`local.HitActorTemp`) "/Game/Characters/Blueprint/Interface/BPI_Interact.BPI_Interact_C") :!label _label
                (set `self.LastCheckInteractActor` (`local.HitActorTemp`))
                (`/Game/Widgets/Gameplay/WB_GameplayContainer.ControlCentralDotState` (`/Game/Characters/Blueprint/Player/PC_BaseController.GameplayContainer` (`self.PC Base Controller`)) true)
                (bind _itemdata (message `/Game/Characters/Blueprint/Interface/BPI_Interact.BPI GetItemData` (`local.HitActorTemp`)))
                (`/Game/Widgets/Gameplay/WB_GameplayContainer.ControlInfoWidget` (`/Game/Characters/Blueprint/Player/PC_BaseController.GameplayContainer` (`self.PC Base Controller`)) true _itemdata))))
          (:`else`
            (goto _label))))
      (:`else`))
    (else
      (`self.LastCheckInteractActor`
        (:`then`
          (set `self.LastCheckInteractActor` null)
          (`/Game/Widgets/Gameplay/WB_GameplayContainer.ControlCentralDotState` (`/Game/Characters/Blueprint/Player/PC_BaseController.GameplayContainer` (`self.PC Base Controller`)) false)
          (`/Game/Widgets/Gameplay/WB_GameplayContainer.ControlInfoWidget` :`self` (`/Game/Characters/Blueprint/Player/PC_BaseController.GameplayContainer` (`self.PC Base Controller`))))
        (:`else`)))))

(fn `CheckInteractActorsTraceSolver`
  (params (Condition :type Boolean))
  (bind _ascharacter (cast `Character` (`self.GetOwner`)))
  (if (`Pawn.IsLocallyControlled` _ascharacter)
    (if Condition
      (bind _returnvalue (`KismetSystemLibrary.K2_SetTimerDelegate` (`|CreateDelegate` :!event `CheckInteractActorsTrace`) 0.3 true))
      (set `self.CheckInteractActorsTraceTimerHandle` _returnvalue)
      (else
        (`KismetSystemLibrary.K2_ClearAndInvalidateTimerHandle` (`self.CheckInteractActorsTraceTimerHandle`))))))

(fn `Control Real Time Character State`
  (params (Selection :type "/Game/Characters/Blueprint/Data/Tables/E_ControlArrayAction Enum" :default "NewEnumerator0") (Tag :type "GameplayTag Structure"))
  (switch `/Game/Characters/Blueprint/Data/Tables/E_ControlArrayAction` Selection
    (:`NewEnumerator0`
      (`BlueprintGameplayTagLibrary.AddGameplayTag` (`self.GameplayTagsContainer`) Tag))
    (:`NewEnumerator1`
      (`BlueprintGameplayTagLibrary.RemoveGameplayTag` (`self.GameplayTagsContainer`) Tag))))

(fn `ControlGrabbedComponentPosition`
  (if (`BlueprintGameplayTagLibrary.HasTag` (`self.GameplayTagsContainer`) (struct :`TagName` "States.Character.Interact.GrabObject"))
    (`self.HeldItem`
      (:`then`
        (`PhysicsHandleComponent.SetTargetLocationAndRotation` (`self.Physics Handle`) (+ (+ (`Actor.K2_GetActorLocation` (`self.Owner`)) (0.0 0.0 44.0)) (* (`KismetMathLibrary.GetForwardVector` (`/Game/Characters/Blueprint/Player/BP_BaseCharacter.ControlRotation` (`self.Owner`))) (`self.GrabbedComponentHoldDistance`))) (`self.HeldActorRotation`)))
      (:`else`))))

(fn `CrouchSolver`
  (params (Condition :type Boolean))
  (`/Engine/EditorBlueprintResources/ActorComponentMacros.Switch Has Authority`
    (:`Authority`
      (`self.Multicast_Crouch` Condition))
    (:`Remote`
      (`self.Server_Crouch` Condition))))

(fn `Deactivate State`
  (params (Tag :type "GameplayTag Structure"))
  (returns (ReturnValue :type Boolean))
  (locals (CurrentState :type "GameplayTag Structure") (States_temp :type "/Game/Characters/Blueprint/Data/Tables/S_CharacterState_Solver Structure"))
  (bind ((`AfterDeactivatingCancelTags_46_AD2F4D1B4EE5416B2FF032A15358940C` _afterdeactivatingcanceltags) (`AfterDeactivatingActivateTags_48_F4786A464E9A12F44CAA4A9D82C84BDD` _afterdeactivatingactivatetags)) (break `/Game/Characters/Blueprint/Data/Tables/S_CharacterState_Solver` (`local.States_temp`)))
  (bind _output_get (set `local.CurrentState` Tag))
  (if (`self.Does State Exist` _output_get)
    (set `local.States_temp` (`self.Get State Structure` (`local.CurrentState`)))
    (`|ExecutionSequence`
      (:`then_0`
        (`self.Cancel State Solver` (`local.CurrentState`)))
      (:`then_1`
        (`self.Control Real Time Character State` "NewEnumerator1" (`local.CurrentState`))
        (`self.Replicate Real Time Character State - Solver` (`self.GameplayTagsContainer`))
        (`self.ActivateStates` (`BlueprintGameplayTagLibrary.BreakGameplayTagContainer` _afterdeactivatingactivatetags))
        (`self.Deactivate States` (`BlueprintGameplayTagLibrary.BreakGameplayTagContainer` _afterdeactivatingcanceltags)))
      (:`then_2`
        (return true)))
    (else
      (return false))))

(fn `Deactivate States`
  (params (Tags :type "Array of GameplayTag Structure"))
  (locals (CurrentState :type "GameplayTag Structure") (States_temp :type "/Game/Characters/Blueprint/Data/Tables/S_CharacterState_Solver Structure"))
  (bind ((`AfterDeactivatingCancelTags_46_AD2F4D1B4EE5416B2FF032A15358940C` _afterdeactivatingcanceltags) (`AfterDeactivatingActivateTags_48_F4786A464E9A12F44CAA4A9D82C84BDD` _afterdeactivatingactivatetags)) (break `/Game/Characters/Blueprint/Data/Tables/S_CharacterState_Solver` (`local.States_temp`)))
  (for _array_element Tags
    (bind _output_get (set `local.CurrentState` _array_element))
    (if (`self.Does State Exist` _output_get)
      (set `local.States_temp` (`self.Get State Structure` (`local.CurrentState`)))
      (`|ExecutionSequence`
        (:`then_0`
          (`self.Cancel State Solver` (`local.CurrentState`)))
        (:`then_1`
          (`self.Control Real Time Character State` "NewEnumerator1" (`local.CurrentState`))
          (`self.Replicate Real Time Character State - Solver` (`self.GameplayTagsContainer`))
          (`self.ActivateStates` (`BlueprintGameplayTagLibrary.BreakGameplayTagContainer` _afterdeactivatingactivatetags))
          (`self.Deactivate States` (`BlueprintGameplayTagLibrary.BreakGameplayTagContainer` _afterdeactivatingcanceltags)))
        (:`then_2`)))))

(fn `Does State Exist`
  (params (Tag :type "GameplayTag Structure"))
  (returns (ReturnValue :type Boolean))
  (return (`BlueprintGameplayTagLibrary.HasTag` (`self.GameplayTagsContainer`) Tag)))

(fn `Get State Structure`
  (params (Tag :type "GameplayTag Structure"))
  (returns (`Out Row` :type "/Game/Characters/Blueprint/Data/Tables/S_CharacterState_Solver Structure"))
  ;[1 1 1] Get State Structure
  (bind _returnvalue (`|GetDataTableRow` "/Game/Characters/Blueprint/Data/Tables/DT_CharacterStates.DT_CharacterStates" (`KismetStringLibrary.Conv_StringToName` (`BlueprintGameplayTagLibrary.GetDebugStringFromGameplayTag` Tag)))
    (:`then`
      (return _returnvalue))))

(fn `GetCharacterMovement`
  (returns (`Character Movement` :type "CharacterMovementComponent Object Reference"))
  (return (`Character.CharacterMovement` (`self.Owner`))))

(fn `GrabObjectSolver`
  (params (Condition :type Boolean))
  (bind (_returnvalue_location _returnvalue_rotation) (`KismetMathLibrary.BreakTransform` (`Actor.GetTransform` (`self.HeldItem`))))
  (if Condition
    (bind _lastinteractactor (`self.LastInteractActor`)
      (:`then`
        (bind _asbp_interact_physic (cast `/Game/Characters/World/Interact/BP_InteractPhysic` _lastinteractactor))
        (bind _output_get (set `self.HeldItem` _asbp_interact_physic))
        (`self.Client_SetGrabObjectRef` _output_get)
        (`/Game/Characters/World/Interact/BP_InteractPhysic.Multicast_SetResponseToCharacter` (`self.HeldItem`) "ECR_Ignore")
        (`PhysicsHandleComponent.GrabComponentAtLocationWithRotation` (`self.Physics Handle`) (`/Game/Characters/World/Interact/BP_InteractMaster.StaticMesh` (`self.HeldItem`)) "None" _returnvalue_location _returnvalue_rotation)
        (`/Game/Characters/World/Interact/BP_InteractPhysic.Multicast_ControlHeldByRef` (`self.HeldItem`) (`self.Owner`))
        (`self.SetComponentTickEnabled` true))
      (:`else`))
    (else
      (`self.HeldItem`
        (:`then`
          (if (`self.DropGrabbedObjectNeedImpulse`)
            (`PhysicsHandleComponent.ReleaseComponent` (`self.Physics Handle`))
            (`PrimitiveComponent.AddImpulse` (`/Game/Characters/World/Interact/BP_InteractMaster.StaticMesh` (`self.HeldItem`)) (* (`KismetMathLibrary.GetForwardVector` (`/Game/Characters/Blueprint/Player/BP_BaseCharacter.ControlRotation` (`self.Owner`))) (`self.ThrowGrabbedObjectStrength`)) "None" true)
            (else
              (`PhysicsHandleComponent.ReleaseComponent` (`self.Physics Handle`))))
          (`/Game/Characters/World/Interact/BP_InteractPhysic.Multicast_ControlHeldByRef` (`self.HeldItem`) null)
          (`/Game/Characters/World/Interact/BP_InteractPhysic.Multicast_SetResponseToCharacter` (`self.HeldItem`) "ECR_Block")
          (set `self.HeldItem` null)
          (`self.Client_SetGrabObjectRef` null)
          (`self.SetComponentTickEnabled` false))
        (:`else`)))))

(fn `IA Crouch`
  (params (Condition :type Boolean))
  (if Condition
    (`self.Activate State` (struct :`TagName` "States.Character.Movement.Crouch"))
    (else
      (`self.Deactivate State` (struct :`TagName` "States.Character.Movement.Crouch")))))

(fn `IA LeftMouseButton`)

(fn `IA MouseWheel`
  (params (Axis :type "Float (double-precision)"))
  (`self.HeldItem`
    (:`then`
      (`self.Server_SetHoldDistanceGrabbedObject` Axis))
    (:`else`)))

(fn `IA_Interact`
  (`self.Activate State` (struct :`TagName` "States.Character.Interact.TryInteract")))

(fn `IA_JumpState`
  (params (Condition :type Boolean))
  (if Condition
    (`self.Activate State` (struct :`TagName` "States.Character.Movement.Jump"))
    (else
      (`self.Deactivate State` (struct :`TagName` "States.Character.Movement.Jump")))))

(fn `IA_RotateGrabbedObject`
  (params (Vector :type "Vector2D Structure"))
  (bind (_x _y) (`KismetMathLibrary.BreakVector2D` Vector))
  (bind (_heldactorrotation_roll _heldactorrotation_pitch _heldactorrotation_yaw) (`KismetMathLibrary.BreakRotator` (`self.HeldActorRotation`)))
  (`self.HeldItem`
    (:`then`
      (bind _output_get (set `self.HeldActorRotation` (`KismetMathLibrary.MakeRotator` (+ _heldactorrotation_roll _y) _heldactorrotation_pitch (+ _heldactorrotation_yaw _x))))
      (`self.Server_SetGrabbedObjectRotation` _output_get))
    (:`else`)))

(fn `IA_RunState`
  (params (Condition :type Boolean))
  (if Condition
    (`self.Activate State` (struct :`TagName` "States.Character.Movement.Run"))
    (else
      (`self.Deactivate State` (struct :`TagName` "States.Character.Movement.Run")))))

(fn `InteractSolver`
  (params (InteractKey :type "/Game/Characters/World/Interact/EInteractActionKey Enum" :default "NewEnumerator3"))
  (bind _lastcheckinteractactor (`self.LastCheckInteractActor`)
    (:`then`
      (`self.Server_Interact` _lastcheckinteractactor InteractKey))
    (:`else`)))

(fn `InteractTrace`
  (returns (HitActor :type "Actor Object Reference") (ReturnValue :type Boolean))
  (bind _returnvalue (`GameplayStatics.GetPlayerController` 0))
  (bind _returnvalue_2 (`Actor.K2_GetActorLocation` (`PlayerController.PlayerCameraManager` _returnvalue)))
  (bind (_outhit _returnvalue_3) (`KismetSystemLibrary.LineTraceSingle` _returnvalue_2 (+ _returnvalue_2 (* (`Actor.GetActorForwardVector` _returnvalue) 500)) (`self.Trace Channel Interact`)))
  (if _returnvalue_3
    (return (`.HitActor` (`GameplayStatics.BreakHitResult` _outhit)) _returnvalue_3)))

(fn `JumpSolver`
  (params (Condition :type Boolean))
  (`/Engine/EditorBlueprintResources/ActorComponentMacros.Switch Has Authority`
    (:`Authority`
      (`self.Multicast_Jump` Condition))
    (:`Remote`
      (`self.Server_Jump` Condition))))

(fn `Replicate Real Time Character State - Solver`
  (params (GameplayTagsContainer :type "GameplayTagContainer Structure"))
  (`/Engine/EditorBlueprintResources/ActorComponentMacros.Switch Has Authority`
    (:`Authority`
      (`self.Replicate_RealTime Character State - ALL` GameplayTagsContainer))
    (:`Remote`
      (`self.Replicate_RealTime Character State - Server` GameplayTagsContainer))))

(fn `RunSolver`
  (params (Condition :type Boolean))
  (`/Engine/EditorBlueprintResources/ActorComponentMacros.Switch Has Authority`
    (:`Authority`
      (`self.Multicast_RunState` Condition))
    (:`Remote`
      (`self.Server_RunState` Condition))))

(fn `State Machine Solver`
  (params (Tag :type "GameplayTag Structure"))
  (returns (StateContainer :type "/Game/Characters/Blueprint/Data/Tables/S_AC_StateContainer Structure"))
  (locals (States_temp :type "/Game/Characters/Blueprint/Data/Tables/S_CharacterState_Solver Structure") (ForbiddenStateFound_temp :type Boolean) (CancelStates :type "GameplayTagContainer Structure"))
  (bind ((`NecessaryTagsForActivating_36_684563CA4ACFBCB1FC15BA971A2B6296` _necessarytagsforactivating) (`ForbiddenTagsForActivating_38_28212EE64317E9C746A628AC483A7A98` _forbiddentagsforactivating) (`AfterActivatingActivateTags_43_FAE6684F41E949F708F30895E1E637F1` _afteractivatingactivatetags) (`AfterActivatingCancelTags_44_0C1970144638FE08DEAA83ADF1E5BA53` _afteractivatingcanceltags) (`AfterDeactivatingCancelTags_46_AD2F4D1B4EE5416B2FF032A15358940C` _afterdeactivatingcanceltags) (`AfterDeactivatingActivateTags_48_F4786A464E9A12F44CAA4A9D82C84BDD` _afterdeactivatingactivatetags) (`BeforeActivatingActivateTags_56_2A7D20F64DC717799986D4B11B35B647` _beforeactivatingactivatetags) (`BeforeActivatingCancelTags_58_0FAFE5E5418D67F255BF80AB70E65917` _beforeactivatingcanceltags) (`RemoveAfterActivation_62_C6122FF1481F2B67845F86AEB2D8A4F2` _removeafteractivation)) (break `/Game/Characters/Blueprint/Data/Tables/S_CharacterState_Solver` (`local.States_temp`)))
  (bind ((`AfterActivatingActivateTags_43_FAE6684F41E949F708F30895E1E637F1` _afteractivatingactivatetags_2) (`AfterActivatingCancelTags_44_0C1970144638FE08DEAA83ADF1E5BA53` _afteractivatingcanceltags_2) (`BeforeActivatingActivateTags_56_2A7D20F64DC717799986D4B11B35B647` _beforeactivatingactivatetags_2) (`BeforeActivatingCancelTags_58_0FAFE5E5418D67F255BF80AB70E65917` _beforeactivatingcanceltags_2) (`RemoveAfterActivation_62_C6122FF1481F2B67845F86AEB2D8A4F2` _removeafteractivation_2)) (break `/Game/Characters/Blueprint/Data/Tables/S_CharacterState_Solver` (`local.States_temp`)))
  ;[0.7 0 1] IMPORTANT NOTE:
  ; This state machine performs a check to see if the next state can be activated.
  (set `local.States_temp` (`self.Get State Structure` Tag))
  (if (`.ProhibitReActivation_64_7F273F7346FCA5202AED95AE7863B90E` (break `/Game/Characters/Blueprint/Data/Tables/S_CharacterState_Solver` (`local.States_temp`)))
    (if (`BlueprintGameplayTagLibrary.HasTag` (`self.GameplayTagsContainer`) (`.CharacterState_30_BB203C29463B4D2D74F45EA89A961B4D` (break `/Game/Characters/Blueprint/Data/Tables/S_CharacterState_Solver` (`local.States_temp`))))
      (return (make `/Game/Characters/Blueprint/Data/Tables/S_AC_StateContainer` false))
      (else
        _)))
  (set `local.ForbiddenStateFound_temp` (`BlueprintGameplayTagLibrary.HasAnyTags` (`self.GameplayTagsContainer`) (`.ForbiddenTagsForActivating_38_28212EE64317E9C746A628AC483A7A98` (break `/Game/Characters/Blueprint/Data/Tables/S_CharacterState_Solver` (`local.States_temp`)))))
  (if (`local.ForbiddenStateFound_temp`)
    (return (make `/Game/Characters/Blueprint/Data/Tables/S_AC_StateContainer` false))
    (elif (`BlueprintGameplayTagLibrary.HasAllTags` (`self.GameplayTagsContainer`) (`.NecessaryTagsForActivating_36_684563CA4ACFBCB1FC15BA971A2B6296` (break `/Game/Characters/Blueprint/Data/Tables/S_CharacterState_Solver` (`local.States_temp`))))
      (if (`.AdditionalCheck_33_67F878024BA585233B2479BFB4617414` (break `/Game/Characters/Blueprint/Data/Tables/S_CharacterState_Solver` (`local.States_temp`)))
        ;;[1 0.5 0] EXPLANATION:
        ;; "Why is the result wrapped in a structure?" - The point is that a pure function is executed as many times as it has output values. That's why it is much better for optimization when a complex pure function has 1 output than several. In this case, it will be executed only once.
        (if (`self.Additional Check By State Type` (`local.Tag`))
          (return (make `/Game/Characters/Blueprint/Data/Tables/S_AC_StateContainer` true _afteractivatingactivatetags_2 _beforeactivatingactivatetags_2 _beforeactivatingcanceltags_2 _afteractivatingcanceltags_2 _removeafteractivation_2))
          (else
            (return (make `/Game/Characters/Blueprint/Data/Tables/S_AC_StateContainer` false))))
        (else
          (return (make `/Game/Characters/Blueprint/Data/Tables/S_AC_StateContainer` true _afteractivatingactivatetags _beforeactivatingactivatetags _beforeactivatingcanceltags _afteractivatingcanceltags _removeafteractivation))))
      (else
        (return (make `/Game/Characters/Blueprint/Data/Tables/S_AC_StateContainer` false))))))