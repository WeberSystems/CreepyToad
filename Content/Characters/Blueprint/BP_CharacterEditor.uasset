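; BP_CharacterEditor is a character preview actor that shows a skin chosen by gender and index through a Blueprint interface event.
; It picks the skin from the male or female list in CharacterSkinContainer and creates a Customizable Object (Mutable) instance from it.
; That single instance feeds both the mesh and face customizable components, which update asynchronously.
; An interface getter exposes the skin's retarget tag, while GetCharacterSkin returns no value.
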(event `/Game/Characters/Blueprint/BPI_Core.BPI SetNewCharacterSkinPreviewActor`
  (params (Gender :type "/Game/Characters/Blueprint/E_GenderTwo Enum" :default "NewEnumerator0") (Index :type Integer))
  (`self.SetNewCharacterSkin` Gender Index))

(fn `BPI GetCharacterSkin`
  (returns (SkinData :type "/Game/Characters/Blueprint/BP_DA_CharSkin Object Reference"))
  (return null))

(fn `BPI GetCharacterSkinTag`
  (returns (Tag :type Name))
  (bind _characterskin (`self.CharacterSkin`)
    (:`then`
      (return (`/Game/Characters/Blueprint/BP_DA_CharSkin.RetargetTag` _characterskin)))
    (:`else`)))

(fn `SetNewCharacterSkin`
  (params (Gender :type "/Game/Characters/Blueprint/E_GenderTwo Enum" :default "NewEnumerator0") (Index :type Integer))
  (bind _characterskincontainer (`self.CharacterSkinContainer`))
  (`self.UpdateCharacterSkin` (`|GetArrayItem` (select `/Game/Characters/Blueprint/E_GenderTwo` Gender :`NewEnumerator0` (`/Game/Characters/Blueprint/Data/Assets/BP_DA_SkinsContainer.Male` _characterskincontainer) :`NewEnumerator1` (`/Game/Characters/Blueprint/Data/Assets/BP_DA_SkinsContainer.Female` _characterskincontainer)) Index)))

(fn `UpdateCharacterSkin`
  (params (CharacterSkin :type "/Game/Characters/Blueprint/BP_DA_CharSkin Object Reference"))
  (locals (Temp :type "CustomizableObjectInstance Object Reference"))
  (bind _output_get (set `self.CharacterSkin` CharacterSkin))
  (bind _returnvalue (`CustomizableObject.CreateInstance` (`/Game/Characters/Blueprint/BP_DA_CharSkin.Cust` _output_get)))
  (set `local.Temp` _returnvalue)
  (`|ExecutionSequence`
    (:`then_0`
      (`CustomizableSkeletalComponent.SetCustomizableObjectInstance` (`self.CustomizableSkeletalMesh`) (`local.Temp`))
      (`CustomizableSkeletalComponent.UpdateSkeletalMeshAsync` (`self.CustomizableSkeletalMesh`) true))
    (:`then_1`
      (`CustomizableSkeletalComponent.SetCustomizableObjectInstance` (`self.CustomizableSkeletalFace`) (`local.Temp`))
      (`CustomizableSkeletalComponent.UpdateSkeletalMeshAsync` (`self.CustomizableSkeletalFace`) true))))

(fn `UserConstructionScript`)