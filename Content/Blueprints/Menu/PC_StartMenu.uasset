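; Start menu player controller that lets the game begin with a chosen character skin.
; On BeginPlay it applies the starting skin to the level's BP_CharacterEditor preview actor, then shows WB_StartMenu with that actor and skin, using UI-only input and a visible cursor.
; It binds an event to the menu's start-game hook.
; StartGameWithInitialData stores the skin in BP_BaseGameInstance and opens the named level.
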(event `self.ReceiveBeginPlay`
  (bind _returnvalue (`GameplayStatics.GetActorOfClass` "/Game/Blueprints/Menu/BP_CharacterEditor.BP_CharacterEditor_C"))
  (`/Game/Blueprints/Menu/BP_CharacterEditor.UpdateCharacterSkin` _returnvalue (`self.StartCharacterSkin`))
  (bind _returnvalue_2 (`|CreateWidget` "/Game/Widgets/Menu/WB_StartMenu.WB_StartMenu_C" null (`self.StartCharacterSkin`) _returnvalue))
  (`UserWidget.AddToViewport` _returnvalue_2 0)
  (add `/Game/Widgets/Menu/WB_StartMenu.StartGame` _returnvalue_2 (`|CreateDelegate` :!event `StartGameWithInitialData`))
  (set `self.bShowMouseCursor` true)
  (`WidgetBlueprintLibrary.SetInputMode_UIOnlyEx` self _returnvalue_2))

(fn `StartGameWithInitialData`
  (params (CharacterSkin :type "/Game/Characters/Blueprint/BP_DA_CharSkin Object Reference") (LevelName :type Name))
  (bind _asbp_base_game_instance (cast `/Game/Blueprints/Game/BP_BaseGameInstance` (`GameplayStatics.GetGameInstance`)))
  (`/Game/Blueprints/Game/BP_BaseGameInstance.CollectCharacterSkinData` _asbp_base_game_instance CharacterSkin)
  (`GameplayStatics.OpenLevel` LevelName))

(fn `UserConstructionScript`)