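; Character preview actor for the menu's character editor, which displays a skin chosen by gender and index.
; An interface event picks the skin from the male or female list in CharacterSkinContainer and passes it to UpdateCharacterSkin.
; That function applies face and body meshes, materials and the anim class, clears the grooms, then maps groom and clothing entries onto their components by key.
; An interface getter exposes the skin's retarget tag.
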(event `/Game/Characters/Blueprint/BPI_Core.BPI SetNewCharacterSkinPreviewActor`
  (params (Gender :type "/Game/Characters/Blueprint/E_GenderTwo Enum" :default "NewEnumerator0") (Index :type Integer))
  (`self.SetNewCharacterSkin` Gender Index))

(fn `BPI GetCharacterSkin`
  (returns (SkinData :type "/Game/Characters/Blueprint/BP_DA_CharSkin Object Reference"))
  (return null))

(fn `BPI GetCharacterSkinTag`
  (returns (Tag :type Name))
  (bind _characterskin (`self.CharacterSkin`)
    (:`then`
      (return (`/Game/Characters/Blueprint/BP_DA_CharSkin.RetargetTag` _characterskin)))
    (:`else`)))

(fn `SetNewCharacterSkin`
  (params (Gender :type "/Game/Characters/Blueprint/E_GenderTwo Enum" :default "NewEnumerator0") (Index :type Integer))
  (bind _characterskincontainer (`self.CharacterSkinContainer`))
  (`self.UpdateCharacterSkin` (`|GetArrayItem` (select `/Game/Characters/Blueprint/E_GenderTwo` Gender :`NewEnumerator0` (`/Game/Characters/Blueprint/Data/Assets/BP_DA_SkinsContainer.Male` _characterskincontainer) :`NewEnumerator1` (`/Game/Characters/Blueprint/Data/Assets/BP_DA_SkinsContainer.Female` _characterskincontainer)) Index)))

(fn `UpdateCharacterSkin`
  (params (NewCharacterSkin :type "/Game/Characters/Blueprint/BP_DA_CharSkin Object Reference"))
  (locals (Temp :type "CustomizableObjectInstance Object Reference"))
  (bind _array (`|MakeArray` (`self.Eyelashes`) (`self.Hair`) (`self.Beard`) (`self.Mustache`) (`self.Fuzz`) (`self.Eyebrows`)))
  (bind _output_get (set `self.CharacterSkin` NewCharacterSkin))
  (`SkeletalMeshComponent.SetSkeletalMeshAsset` (`self.Face`) (`/Game/Characters/Blueprint/BP_DA_CharSkin.Face` _output_get))
  (for (_array_element _array_index) (`SkeletalMesh.Materials` (`/Game/Characters/Blueprint/BP_DA_CharSkin.Face` _output_get))
    (`PrimitiveComponent.SetMaterial` (`self.Face`) _array_index (break `SkeletalMaterial` _array_element)))
  (`SkeletalMeshComponent.SetSkeletalMeshAsset` (`self.Body`) (`/Game/Characters/Blueprint/BP_DA_CharSkin.Body` (`self.CharacterSkin`)))
  (for (_array_element_2 _array_index_2) (`SkeletalMesh.Materials` (`/Game/Characters/Blueprint/BP_DA_CharSkin.Body` (`self.CharacterSkin`)))
    (`PrimitiveComponent.SetMaterial` (`self.Body`) _array_index_2 (break `SkeletalMaterial` _array_element_2)))
  (`SkeletalMeshComponent.SetAnimInstanceClass` (`self.Body`) "/Game/Characters/ABP/ABP_FirstPersonSK.ABP_FirstPersonSK_C")
  (`|ExecutionSequence`
    (:`then_0`
      (`GroomComponent.SetGroomAsset` _array null)
      (`GroomComponent.SetBindingAsset` _array null)
      (bind _keys (`BlueprintMapLibrary.Map_Keys` (`/Game/Characters/Blueprint/BP_DA_CharSkin.Groom` (`self.CharacterSkin`))))
      (for (_array_element_3 _array_index_3) _keys
        (bind _values (`BlueprintMapLibrary.Map_Values` (`/Game/Characters/Blueprint/BP_DA_CharSkin.Groom` (`self.CharacterSkin`))))
        (bind (_output_groomasset _output_groombinding) (break `/Game/Characters/Blueprint/FGroomData` (`|GetArrayItem` _values _array_index_3)))
        (`GroomComponent.SetGroomAsset` (select `/Game/Characters/Blueprint/EGroomTypes` _array_element_3 :`NewEnumerator0` (`self.Eyelashes`) :`NewEnumerator1` (`self.Hair`) :`NewEnumerator2` (`self.Beard`) :`NewEnumerator3` (`self.Mustache`) :`NewEnumerator4` (`self.Fuzz`) :`NewEnumerator5` (`self.Eyebrows`)) _output_groomasset)
        (`GroomComponent.SetBindingAsset` (`self.Eyelashes`) _output_groombinding)
        (`GroomComponent.SetBindingAsset` (select `/Game/Characters/Blueprint/EGroomTypes` _array_element_3 :`NewEnumerator0` (`self.Eyelashes`) :`NewEnumerator1` (`self.Hair`) :`NewEnumerator2` (`self.Beard`) :`NewEnumerator3` (`self.Mustache`) :`NewEnumerator4` (`self.Fuzz`) :`NewEnumerator5` (`self.Eyebrows`)) _output_groombinding)))
    (:`then_1`
      (bind _keys_2 (`BlueprintMapLibrary.Map_Keys` (`/Game/Characters/Blueprint/BP_DA_CharSkin.BodyParts` (`self.CharacterSkin`))))
      (for (_array_element_4 _array_index_4) _keys_2
        (bind _values_2 (`BlueprintMapLibrary.Map_Values` (`/Game/Characters/Blueprint/BP_DA_CharSkin.BodyParts` (`self.CharacterSkin`))))
        (bind _returnvalue (select `/Game/Characters/Blueprint/EBodyParts` _array_element_4 :`NewEnumerator0` (`self.Top`) :`NewEnumerator1` (`self.Buttom`) :`NewEnumerator2` (`self.Shoes`)))
        (`SkeletalMeshComponent.SetSkeletalMeshAsset` _returnvalue (`|GetArrayItem` _values_2 _array_index_4))
        (`SceneComponent.SetHiddenInGame` _returnvalue (== _returnvalue null) false)))))

(fn `UserConstructionScript`)